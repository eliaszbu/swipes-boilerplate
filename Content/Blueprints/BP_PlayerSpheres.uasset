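; BP_PlayerSpheres exposes a lookup that maps an event value to one of five player spheres: Left, Right, Top, Bottom or Middle.
; GetSphereByEventValue selects on the vertical axis when X is zero, otherwise on the horizontal axis.
; The truncated component indexes a Select, with a +1 offset applied only to Y, so the two axes expect different value ranges.
; The event graph and construction script are empty.
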(fn `GetSphereByEventValue`
  (params (Value :type "Vector2D Structure"))
  (returns (ReturnValue :type "StaticMeshComponent Object Reference"))
  (if (== Value_X 0.0)
    (return (select `int` (+ (`KismetMathLibrary.FTrunc` Value_Y) 1) :`0` (`self.Bottom`) :`1` (`self.Middle`) :`2` (`self.Top`)))
    (else
      (return (select `int` (`KismetMathLibrary.FTrunc` Value_X) :`0` (`self.Left`) :`1` (`self.Middle`) :`2` (`self.Right`))))))

(fn `UserConstructionScript`)